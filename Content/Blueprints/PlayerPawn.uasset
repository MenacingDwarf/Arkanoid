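; Player paddle pawn for a brick-breaker game that also manages score, lives, combo, HUD and game over.
; Left/Right input moves it and any unlaunched ball, which Space launches.
; Every fifth paddle hit has BlockGenerator spawn a line, while score milestones add lives or speed up the ball.
; The ball's OnDead event clears blocks past an X threshold and costs a life, respawning or returning to MenuMap.
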(event Custom|GetScores
  (params (Scores :type Integer))
  ;[1 1 1] Обновление очков
  (Variables|Default|SetScores (+ (Variables|Default|GetScores) Scores))
  (if (== (Math|Integer|%(Integer) (Variables|Default|GetScores) 50) 0)
    (CallFunction|AddLive))
  (CallFunction|UpdateScores)
  (if (== (Math|Integer|%(Integer) (Variables|Default|GetScores) 5) 0)
    (CallFunction|SpeedUp)))

(event Custom|UpdateScores
  ;[1 1 1] Обновление очков
  (Rendering|Components|TextRender|SetText (Variables|/Game/Widgets/MainWB.MainWB_C|GetScores_TextBox (Variables|Default|GetMainWB)) (Utilities|Text|ToText(Integer) (Variables|Default|GetScores))))

(event Custom|Death
  ;[1 1 1] Спавн меча и смерть
  (CallFunction|DestroyBlocks)
  (Variables|Default|SetBall%20Hits 0)
  (Actor|DestroyActor (Variables|Default|GetBallRef))
  (CallFunction|ReduceLives)
  (if (or (<= (Variables|Default|GetLives) 0) (Variables|Default|GetIs%20Dead?))
    (CallFunction|GameOver)
    (else
      (CallFunction|SpawnBall)
      (Widget|SetVisibility (Variables|/Game/Widgets/MainWB.MainWB_C|GetSpace_SizeBox (Variables|Default|GetMainWB)) "Visible"))))

(event Custom|Spawn%20Ball
  ;[1 1 1] Спавн меча и смерть
  (bind _returnvalue (Game|SpawnActorfromClass "/Game/Blueprints/Ball.Ball_C" (Math|Transform|MakeTransform (Transformation|GetWorldLocation (Variables|Default|GetBall%20Position)) "0, 0, 0" "0.700000,0.700000,0.700000") "Undefined" 0 (Variables|Default|GetBall%20Speed) self 0))
  (bind _output_get (Variables|Default|SetBallRef _returnvalue))
  (EventDispatchers|BindEventtoOnDead _output_get (delegate Custom|Death)))

(event Custom|Update%20Lives
  ;[1 1 1] Обновление очков
  (Rendering|Components|TextRender|SetText (Variables|/Game/Widgets/MainWB.MainWB_C|GetLives_TextBox (Variables|Default|GetMainWB)) (Utilities|Text|ToText(Integer) (Variables|Default|GetLives))))

(event Custom|Add%20Live
  ;[1 1 1] Обновление очков
  (Variables|Default|SetLives (+ (Variables|Default|GetLives) 1))
  (CallFunction|UpdateLives))

(event Custom|Reduce%20Lives
  ;[1 1 1] Обновление очков
  (Variables|Default|SetLives (- (Variables|Default|GetLives) 1))
  (CallFunction|UpdateLives))

(event Custom|Update%20Combo
  (params (New%20Combo :type Integer) (Increase :type Boolean))
  ;[1 1 1] Комбо
  (if Increase
    (Math|Integer|IncrementInt (Variables|Default|GetCurrentCombo)
      (:%20%20
        _))
    (else
      (bind _output_get (Variables|Default|SetCurrentCombo New%20Combo))))
  (Rendering|Components|TextRender|SetText (Variables|/Game/Widgets/MainWB.MainWB_C|GetCombo_TextBox_1 (Variables|Default|GetMainWB)) (Utilities|Text|FormatText "x{combo}" _output_get))
  (Widget|SetVisibility (Variables|/Game/Widgets/MainWB.MainWB_C|GetCombo_sizeBox (Variables|Default|GetMainWB)) (select (>= (Variables|Default|GetCurrentCombo) 2) "Visible" "Hidden")))

(event Custom|GameOver
  ;[1 1 1] Game Over
  (Utilities|IsValid (Variables|Default|GetBallRef)
    (:Is%20Valid
      (Actor|DestroyActor (Variables|Default|GetBallRef)))
    (:Is%20Not%20Valid
      _))
  (Variables|Default|SetIs%20Dead? true)
  (Variables|Default|SetDirection "0, 0, 0")
  (Widget|SetVisibility (Variables|/Game/Widgets/MainWB.MainWB_C|GetGameOver_sizeBox (Variables|Default|GetMainWB)) "Visible")
  (Utilities|FlowControl|Delay 2.0)
  (Game|OpenLevel(byName) "MenuMap"))

(event EventBeginPlay
  ;[1 1 1] Hit/Tick/BeginPlay
  (Variables|Default|SetDirection "0, 0, 0")
  (bind _returnvalue (UserInterface|CreateWidget "/Game/Widgets/MainWB.MainWB_C" (Game|GetPlayerController 0)))
  (bind _output_get (Variables|Default|SetMainWB _returnvalue))
  (UserInterface|Viewport|AddtoViewport _output_get 0)
  (CallFunction|UpdateScores)
  (CallFunction|UpdateLives)
  (bind _outactors (Actor|GetAllActorsOfClass "/Game/Blueprints/BlockGenerator.BlockGenerator_C"))
  (Variables|Default|SetBlockGeneratorRef (Utilities|Array|Get(acopy) _outactors))
  (CallFunction|SpawnBall))

(event EventTick
  (params (DeltaSeconds :type Float%20%28single-precision%29))
  (bind _speed (Variables|Default|GetSpeed))
  (bind _direction (Variables|Default|GetDirection))
  (bind _returnvalue (* DeltaSeconds _speed))
  (bind _returnvalue_2 (* _direction _returnvalue))
  ;[1 1 1] Hit/Tick/BeginPlay
  (Transformation|AddActorWorldOffset _returnvalue_2 true)
  (Utilities|IsValid (Variables|Default|GetBallRef)
    (:Is%20Valid
      (if (not (Variables|/Game/Blueprints/Ball.Ball_C|GetStarted (Variables|Default|GetBallRef)))
        (Transformation|AddActorWorldOffset (Variables|Default|GetBallRef) _returnvalue_2 true)))))

(event Collision|EventHit
  (params (MyComp :type Primitive%20Component%20Object%20Reference) (Other :type Actor%20Object%20Reference) (OtherComp :type Primitive%20Component%20Object%20Reference) (bSelfMoved :type Boolean) (HitLocation :type Vector :default "0, 0, 0") (HitNormal :type Vector :default "0, 0, 0") (NormalImpulse :type Vector :default "0, 0, 0") (Hit :type Hit%20Result%20Structure%20%28by%20ref%29))
  ;[1 1 1] Hit/Tick/BeginPlay
  (Utilities|Casting|CastToBall Other)
  (CallFunction|UpdateCombo 0 false)
  (bind _output_get (Variables|Default|SetBall%20Hits (+ (Variables|Default|GetBall%20Hits) 1)))
  (if (== (Math|Integer|%(Integer) _output_get 5) 0)
    (Variables|Default|SetBall%20Hits 0)
    (Default|SpawnLine (Variables|Default|GetBlockGeneratorRef))))

(event Input|ActionEvents|InputActionRight
  (params (Key :type Key%20Structure :default "None"))
  ;[1 1 1] Нажатие клавиш
  (:Pressed
    (if (not (Variables|Default|GetIs%20Dead?))
      (Variables|Default|SetDirection "0.000000,1.000000,0.000000")))
  (:Released
    (if (Class|KismetMathLibrary|EqualExactlyVectorVector (Variables|Default|GetDirection) "0,1.000000, 0")
      (Variables|Default|SetDirection "0, 0, 0"))))

(event Input|ActionEvents|InputActionLeft
  (params (Key :type Key%20Structure :default "None"))
  ;[1 1 1] Нажатие клавиш
  (:Pressed
    (if (not (Variables|Default|GetIs%20Dead?))
      (Variables|Default|SetDirection "0.000000,-1.000000, 0")))
  (:Released
    (if (Class|KismetMathLibrary|EqualExactlyVectorVector (Variables|Default|GetDirection) "0,-1.000000, 0")
      (Variables|Default|SetDirection "0, 0, 0"))))

(event Input|KeyboardEvents|SpaceBar
  (params (Key :type Key%20Structure :default "None"))
  ;[1 1 1] Нажатие клавиш
  (:Pressed
    (Utilities|IsValid (Variables|Default|GetBallRef)
      (:Is%20Valid
        (if (not (Variables|/Game/Blueprints/Ball.Ball_C|GetStarted (Variables|Default|GetBallRef)))
          (Default|ChangeDirection (Variables|Default|GetBallRef) (Math|Rotator|MakeRotator 0.0 0.0 (* 60 (.y (Variables|Default|GetDirection)))))
          (Variables|/Game/Blueprints/Ball.Ball_C|SetStarted (Variables|Default|GetBallRef) true)
          (Widget|SetVisibility (Variables|/Game/Widgets/MainWB.MainWB_C|GetSpace_SizeBox (Variables|Default|GetMainWB)) "Hidden"))))))

(fn ConstructionScript)

(fn SpeedUp
  (if (< (Variables|Default|GetBall%20Speed) 1.2e+03)
    (Variables|Default|SetBall%20Speed (+ (Variables|Default|GetBall%20Speed) 5e+01))
    (Default|SpeedUp (Variables|Default|GetBallRef))))

(fn DestroyBlocks
  (bind _outactors (Actor|GetAllActorsOfClass "/Game/Blueprints/Block.Block_C"))
  (for _array_element _outactors
    (if (< (.x (Transformation|GetWorldLocation (Variables|/Game/Blueprints/Block.Block_C|GetCube _array_element))) -2e+02)
      (Actor|DestroyActor _array_element))))