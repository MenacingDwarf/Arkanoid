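; Breakable block for a ball-and-brick game that shows its remaining lives as text and as one of three materials.
; A ball hit plays a sound, awards score and combo to the ball's player pawn, and removes a life.
; At zero lives it notifies its generator with its line, spawns an explosion and destroys itself.
; Otherwise it refreshes text and material, then briefly flashes the ball material with text hidden.
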(event Custom|UpdateLives
  (Rendering|Components|TextRender|SetText (Variables|Default|GetTextRender) (Utilities|Text|ToText(Integer) (Variables|Default|GetLives))))

(event Custom|Update%20Materials
  (switch int (Variables|Default|GetLives)
    (:1
      (Rendering|Material|SetMaterial (Variables|Default|GetCube) 0 "/Game/Materials/Block1Mat.Block1Mat"))
    (:2
      (Rendering|Material|SetMaterial (Variables|Default|GetCube) 0 "/Game/Materials/Block2Mat.Block2Mat"))
    (:3
      (Rendering|Material|SetMaterial (Variables|Default|GetCube) 0 "/Game/Materials/Block3Mat.Block3Mat"))))

(event EventBeginPlay
  (CallFunction|UpdateLives)
  (CallFunction|UpdateMaterials))

(event Collision|EventHit
  (params (MyComp :type Primitive%20Component%20Object%20Reference) (Other :type Actor%20Object%20Reference) (OtherComp :type Primitive%20Component%20Object%20Reference) (bSelfMoved :type Boolean) (HitLocation :type Vector :default "0, 0, 0") (HitNormal :type Vector :default "0, 0, 0") (NormalImpulse :type Vector :default "0, 0, 0") (Hit :type Hit%20Result%20Structure%20%28by%20ref%29))
  (bind _asball (Utilities|Casting|CastToBall Other))
  (Audio|PlaySoundatLocation "/Game/Effects/sempl-sintezatora-dabstep-royal-synth__Pro-Sound__mp3cut_net___1___1__Cue.sempl-sintezatora-dabstep-royal-synth__Pro-Sound__mp3cut_net___1___1__Cue" "0, 0, 0" "0, 0, 0" 1.0 1.0 0.0 0 0 0)
  (Default|GetScores (Variables|/Game/Blueprints/Ball.Ball_C|GetPlayerPawn _asball) 1)
  (Default|UpdateCombo (Variables|/Game/Blueprints/Ball.Ball_C|GetPlayerPawn _asball) 0 true)
  (bind _output_get (Variables|Default|SetLives (- (Variables|Default|GetLives) 1)))
  (if (<= _output_get 0)
    (Default|BlockDestroyed (Variables|Default|GetGenerator%20Ref) (Variables|Default|GetLine))
    (Effects|SpawnEmitteratLocation "/Game/StarterContent/Particles/P_Explosion.P_Explosion" HitLocation)
    (Actor|DestroyActor)
    (else
      (CallFunction|UpdateLives)
      (CallFunction|UpdateMaterials)
      (Utilities|LightBlockfor0,1))))

(fn ConstructionScript)