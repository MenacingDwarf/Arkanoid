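; Bonus is a moving pickup actor that grants a bonus to the player pawn on contact.
; At BeginPlay it caches the Sphere component's forward vector as its direction, then moves along it each tick at Speed without sweeping.
; On overlapping a PlayerPawn it calls that pawn's GetBonus and destroys itself, leaving the effect of the bonus to the pawn.
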(event Collision|EventActorBeginOverlap
  (params (OtherActor :type Actor%20Object%20Reference))
  (bind _asplayer_pawn (Utilities|Casting|CastToPlayerPawn OtherActor))
  (Default|GetBonus _asplayer_pawn)
  (Actor|DestroyActor))

(event EventBeginPlay
  (Variables|Default|SetDirection (Math|Rotator|GetRotationXVector (Transformation|GetWorldRotation (Variables|Default|GetSphere)))))

(event EventTick
  (params (DeltaSeconds :type Float%20%28single-precision%29))
  (Transformation|AddActorWorldOffset (* (* (Variables|Default|GetDirection) (Variables|Default|GetSpeed)) DeltaSeconds)))

(fn ConstructionScript)