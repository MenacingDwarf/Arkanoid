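; Ball actor that bounces around the level once started, deflected by the player pawn and other blocking surfaces.
; Tick moves it with a swept offset along Direction at Speed, reflecting off hit normals and calling OnDead on a DeadWall hit.
; Player hits blend the pawn's normalized Direction into the bounce, letting the player influence the angle.
; SpeedUp raises speed up to a limit, and ChangeDirection re-aims the ball from a given rotation.
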(event Custom|SpeedUp
  (if (< (Variables|Default|GetSpeed) 1.2e+03)
    (Variables|Default|SetSpeed (+ (Variables|Default|GetSpeed) 5e+01))))

(event EventBeginPlay
  (Variables|Default|SetDirection (Math|Rotator|GetRotationXVector (Transformation|GetActorRotation))))

(event EventTick
  (params (DeltaSeconds :type Float%20%28single-precision%29))
  (if (Variables|Default|GetStarted)
    (bind _sweephitresult (Transformation|AddActorWorldOffset (* (Variables|Default|GetDirection) (* (Variables|Default|GetSpeed) DeltaSeconds)) true))
    (Utilities|Casting|CastToDeadWall (.HitActor (Collision|BreakHitResult _sweephitresult))
      (:then
        (Default|CallOnDead))
      (:CastFailed
        (Utilities|Casting|CastToPlayerPawn (.HitActor (Collision|BreakHitResult _sweephitresult))
          (:then
            (bind _output_get (Variables|Default|SetDirection (Math|Vector|Normalize (+ (Math|Vector|GetReflectionVector (Variables|Default|GetDirection) (.Normal (Collision|BreakHitResult _sweephitresult))) (Math|Vector|Normalize (Variables|/Game/Blueprints/PlayerPawn.PlayerPawn_C|GetDirection (.AsPlayer%20Pawn (Utilities|Casting|CastToPlayerPawn (Game|Player|GetPlayerPawn 0)))))))))
            (Transformation|SetActorRotation (Math|Conversions|RotationFromXVector _output_get)))
          (:CastFailed
            (if (.bBlockingHit (Collision|BreakHitResult _sweephitresult))
              (bind _output_get_2 (Variables|Default|SetDirection (Math|Vector|GetReflectionVector (Variables|Default|GetDirection) (.Normal (Collision|BreakHitResult _sweephitresult)))))
              (Transformation|SetActorRotation (Math|Conversions|RotationFromXVector _output_get_2)))))))))

(fn ConstructionScript)

(fn ChangeDirection
  (params (Vector :type Rotator))
  (Transformation|SetActorRotation Vector)
  (Variables|Default|SetDirection (Math|Rotator|GetRotationXVector Vector)))