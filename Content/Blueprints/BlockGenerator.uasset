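; Block generator actor that spawns and advances rows of destructible blocks toward a losing boundary.
; Spawns two rows at start; each new row first shifts every block back along X by one block size, then fills slots with random-life blocks or gaps.
; After each row, any block past a fixed X limit triggers the player pawn's death.
; BlockDestroyed spawns another row when only one block actor remains.
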(event Custom|Spawn%20Line
  (CallFunction|SpawnNewLine))

(event EventBeginPlay
  (for _index (range 1 2)
    (CallFunction|SpawnLine)))

(fn ConstructionScript)

(fn MoveAllBlocks
  (bind _outactors (Actor|GetAllActorsOfClass "/Game/Blueprints/Block.Block_C"))
  (for _array_element _outactors
    (CallFunction|MoveBlock _array_element)))

(fn MoveBlock
  (params (Block :type Block%20Object%20Reference))
  (Transformation|AddActorWorldOffset Block (Math|Vector|MakeVector (* (Variables|Default|GetBlockSize) -1.0) 0.0 0.0)))

(fn SpawnNewLine
  (bind _returnvalue (Transformation|GetActorLocation))
  (Variables|Default|SetX (+ (Variables|Default|GetX) 1))
  (CallFunction|MoveAllBlocks)
  (for _index (range 1 (Variables|Default|GetY))
    (bind _output_get (LocalVariables|SetLocal%20Lives (Math|Random|RandomIntegerinRange 0 3)))
    (if (!= _output_get 0)
      (Game|SpawnActorfromClass "/Game/Blueprints/Block.Block_C" (Math|Transform|MakeTransform (Math|Vector|MakeVector (- (.x _returnvalue) (.x (* (Math|Vector|MakeVector 1.0 (Math|Conversions|ToFloat(Integer) _index) 0.5) (Variables|Default|GetBlockSize)))) (+ (.y _returnvalue) (.y (* (Math|Vector|MakeVector 1.0 (Math|Conversions|ToFloat(Integer) _index) 0.5) (Variables|Default|GetBlockSize)))) (.z (* (Math|Vector|MakeVector 1.0 (Math|Conversions|ToFloat(Integer) _index) 0.5) (Variables|Default|GetBlockSize)))) "0, 0, 0" "1,1,1") "Undefined" 0 (LocalVariables|GetLocal%20Lives) (Variables|Default|GetX) self 0)
      (LocalVariables|SetBlock%20In%20Line (+ (LocalVariables|GetBlock%20In%20Line) 1))))
  (CallFunction|CheckBlocks))

(fn BlockDestroyed
  (params (Line :type Integer))
  (bind _outactors (Actor|GetAllActorsOfClass "/Game/Blueprints/Block.Block_C"))
  (if (== (Utilities|Array|Length _outactors) 1)
    (CallFunction|SpawnLine)))

(fn CheckBlocks
  (bind _outactors (Actor|GetAllActorsOfClass "/Game/Blueprints/Block.Block_C"))
  (bind _array_element (Utilities|Array|ForEachLoopwithBreak _outactors :!label _label)
    (:LoopBody
      (if (< (.x (Transformation|GetWorldLocation (Variables|/Game/Blueprints/Block.Block_C|GetCube _array_element))) -3.5e+02)
        (Default|Death (.AsPlayer%20Pawn (Utilities|Casting|CastToPlayerPawn (Game|Player|GetPlayerPawn 0))))
        (goto _label Break)))))